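; Robot arm actor built on a PoseableMesh, set up as an experiment in procedurally rotating its joints.
; BeginPlay caches the J2, J3 and J4 bone rotations; the YawLeft and YawRight inputs only print their names.
; Disconnected logic, which never runs, would pitch J2, J3 and J5 within clamps according to a ZToggle flip-flop, and attach GrabSphere actors at joint sockets.
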(event EventBeginPlay
  (bind _poseablemesh (Variables|Default|GetPoseableMesh))
  ;[1 1 1] Get Initial Rotation of J2 Joint
  (bind _returnvalue (Class|PoseableMeshComponent|GetBoneTransformbyName _poseablemesh "J2" "WorldSpace"))
  (bind _output_get (Variables|Default|SetJ2_Initial (.rotation _returnvalue)))
  (bind _output_get_2 (Variables|Default|SetJ2_Iniitial_Split _output_get))
  (bind _returnvalue_2 (Class|PoseableMeshComponent|GetBoneTransformbyName _poseablemesh "J3" "WorldSpace"))
  (bind _output_get_3 (Variables|Default|SetJ3_Initial (.rotation _returnvalue_2)))
  (bind _output_get_4 (Variables|Default|SetJ3_Split _output_get_3))
  (bind _returnvalue_3 (Class|PoseableMeshComponent|GetBoneTransformbyName _poseablemesh "J4" "ComponentSpace"))
  (bind _output_get_5 (Variables|Default|SetJ4_Initial (.rotation _returnvalue_3)))
  (Variables|Default|SetJ4_Split _output_get_5))

(event Collision|EventActorBeginOverlap
  (params (OtherActor :type Actor%20Object%20Reference)))

(event EventTick
  (params (DeltaSeconds :type Float%20%28single-precision%29)))

(event Input|ActionEvents|InputActionYawLeft
  (params (Key :type Key%20Structure :default "None"))
  (:Pressed
    (Development|PrintString "YawLeft")))

(event Input|ActionEvents|InputActionYawRight
  (params (Key :type Key%20Structure :default "None"))
  (:Pressed
    (Development|PrintString "YawRight")))

(event Input|ActionEvents|InputActionzToggle
  (params (Key :type Key%20Structure :default "None")))

(fn ConstructionScript)